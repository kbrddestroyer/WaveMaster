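; BP_WMPlayerController is a player controller that creates the game's action panel, main menu and pause menu widgets.
; On BeginPlay it adds the action panel, then hides it if visible, pauses the game and opens the main menu.
; A pause menu event toggles the panel, pauses and adds the pause menu to the player screen.
; Panel visibility flips through a shared helper that casts the stored widget reference.
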(event `self.ReceiveBeginPlay`
  (`self.AddActionsMenuToScreen`)
  (`self.AddMainMenuToScreen`))

(event `AddMainMenuToScreen`
  (bind _aswbp_action_panel (cast `/Game/Blueprints/UI/WBP_ActionPanel` (`self.CurrActionPanelWidget`)))
  (if (`/Game/Blueprints/UI/WBP_ActionPanel.IsVisibleNow` _aswbp_action_panel)
    (`self.ChangeActionPanelVisibilityIfSet`))
  (`GameplayStatics.SetGamePaused` true)
  (bind _returnvalue (`|CreateWidget` "/Game/Blueprints/UI/WBP_MainMenu.WBP_MainMenu_C"))
  (`UserWidget.AddToViewport` _returnvalue 0))

(event `AddActionsMenuToScreen`
  (bind _returnvalue (`|CreateWidget` "/Game/Blueprints/UI/WBP_ActionPanel.WBP_ActionPanel_C"))
  (bind _output_get (set `self.CurrActionPanelWidget` _returnvalue))
  (`UserWidget.AddToViewport` _output_get 0))

(event `AddPauseMenuToScreen`
  (`self.ChangeActionPanelVisibilityIfSet`)
  (`GameplayStatics.SetGamePaused` true)
  (bind _returnvalue (`|CreateWidget` "/Game/Blueprints/UI/WBP_PauseMenu.WBP_PauseMenu_C"))
  (`UserWidget.AddToPlayerScreen` _returnvalue 0))

(fn `ChangeActionPanelVisibilityIfSet`
  (bind _aswbp_action_panel (cast `/Game/Blueprints/UI/WBP_ActionPanel` (`self.CurrActionPanelWidget`)))
  (`/Game/Blueprints/UI/WBP_ActionPanel.SetVisible` _aswbp_action_panel (not (`/Game/Blueprints/UI/WBP_ActionPanel.IsVisibleNow` _aswbp_action_panel))))

(fn `UserConstructionScript`)